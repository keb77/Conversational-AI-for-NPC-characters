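; Inspection actor for readable items: shows a given mesh to a scene capture with a name and description widget while player input is disabled.
; Dragging with the left mouse rotates the mesh, and the wheel zooms by changing the capture's clamped FOV.
; Space removes the widget and spawns a far-off BP_ReadItem with the title and content; Interact just closes.
; Both exits restore player input and destroy the actor.
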(event Custom|Set%20Rotation%20and%20Scale
  (params (Rotation :type Rotator) (Scale :type Vector))
  (bind _mesh (Variables|Default|GetMesh))
  ;[0.08854 0.08854 0.08854] Set Rotation and Scale
  (bind _output_get (Variables|Default|SetRotation Rotation))
  (bind _output_get_2 (Variables|Default|SetScale Scale))
  (Transformation|SetWorldTransform _mesh (Math|Transform|MakeTransform (.location (Transformation|GetWorldTransform _mesh)) _output_get _output_get_2) false false))

(event Input|EnhancedActionEvents|EnhancedInputActionIA_Interact
  (params (ActionValue :type Boolean) (ElapsedSeconds :type Float%20%28double-precision%29) (TriggeredSeconds :type Float%20%28double-precision%29) (InputAction :type Input%20Action%20Object%20Reference :default "/Game/Game/Input/Actions/IA_Interact.IA_Interact"))
  (bind _returnvalue (Game|GetPlayerController 0))
  ;[0.1042 0.1042 0.1042] Close Widget
  (Input|DisableInput _returnvalue)
  (Input|EnableInput (Variables|Default|GetPlayer) _returnvalue)
  (Utilities|IsValid (Variables|Default|GetInspect%20Widget)
    (:Is%20Valid
      (Widget|RemovefromParent (Variables|Default|GetInspect%20Widget))
      (Variables|Default|SetInspect%20Widget 0)
      (Actor|DestroyActor))))

(event EventInspectRead
  (params (Player :type Character%20Object%20Reference) (Mesh :type Static%20Mesh%20Object%20Reference) (Name :type Text) (Description :type Text) (Title :type Text) (Content :type Text))
  (bind _returnvalue (Game|GetPlayerController 0))
  ;[0.1146 0.1146 0.1146] Create Widget
  (Variables|Default|SetTitle Title)
  (Variables|Default|SetContent Content)
  (Variables|Default|SetPlayer Player)
  (Components|StaticMesh|SetStaticMesh (Variables|Default|GetMesh) Mesh)
  (bind _returnvalue_2 (UserInterface|CreateWidget "/Game/UI/Interact/Inspect/W_InspectReadItem.W_InspectReadItem_C" 0 Name Description))
  (bind _output_get (Variables|Default|SetInspect%20Widget _returnvalue_2))
  (UserInterface|Viewport|AddtoViewport _output_get 0)
  (Input|DisableInput (Variables|Default|GetPlayer) _returnvalue)
  (Input|EnableInput _returnvalue))

(event Input|MouseEvents|MouseX
  (params (AxisValue :type Float%20%28single-precision%29))
  (bind _mesh (Variables|Default|GetMesh))
  ;[0.1667 0.1667 0.1667] Move Item
  (if (Variables|Default|GetRotate?)
    (Transformation|SetWorldRotation _mesh (Math|Rotator|CombineRotators (Transformation|GetWorldRotation _mesh) (Math|Rotator|MakeRotator 0.0 0.0 (* AxisValue -3.0))) false false)))

(event Input|MouseEvents|MouseY
  (params (AxisValue :type Float%20%28single-precision%29))
  (bind _mesh (Variables|Default|GetMesh))
  ;[0.1667 0.1667 0.1667] Move Item
  (if (Variables|Default|GetRotate?)
    (Transformation|SetWorldRotation _mesh (Math|Rotator|CombineRotators (Transformation|GetWorldRotation _mesh) (Math|Rotator|MakeRotator 0.0 (* AxisValue -3.0) 0.0)) false false)))

(event Input|MouseEvents|LeftMouseButton
  (params (Key :type Key%20Structure :default "None"))
  ;[0.1667 0.1667 0.1667] Move Item
  (:Pressed
    (Variables|Default|SetRotate? true))
  (:Released
    (Variables|Default|SetRotate? false)))

(event Input|KeyboardEvents|SpaceBar
  (params (Key :type Key%20Structure :default "None"))
  (bind _returnvalue (Game|GetPlayerController 0))
  ;[0.1042 0.1042 0.1042] Open Read Widget
  (:Pressed
    (Input|DisableInput _returnvalue)
    (Input|EnableInput (Variables|Default|GetPlayer) _returnvalue)
    (Utilities|IsValid (Variables|Default|GetInspect%20Widget)
      (:Is%20Valid
        (Widget|RemovefromParent (Variables|Default|GetInspect%20Widget))
        (Variables|Default|SetInspect%20Widget 0)
        (bind _returnvalue_2 (Game|SpawnActorfromClass "/Game/Game/Blueprints/Interact/BP_ReadItem.BP_ReadItem_C" (Math|Transform|MakeTransform "100000000.000000,0.000000,0.000000") "Undefined" "MultiplyWithRoot" 0 0))
        (Default|Read _returnvalue_2 (Variables|Default|GetPlayer) (Variables|Default|GetTitle) (Variables|Default|GetContent))
        (Actor|DestroyActor)))))

(event Input|MouseEvents|MouseWheelDown
  (params (Key :type Key%20Structure :default "None"))
  (bind _scenecapturecomponent2d (Variables|Default|GetSceneCaptureComponent2D))
  ;[0.1667 0.1667 0.1667] Move Item
  (:Pressed
    (Variables|/Script/Engine.SceneCaptureComponent2D|SetFOVAngle _scenecapturecomponent2d (Math|Float|Clamp(Float) (+ (Variables|/Script/Engine.SceneCaptureComponent2D|GetFOVAngle _scenecapturecomponent2d) 3.0) 3e+01 8e+01))))

(event Input|MouseEvents|MouseWheelUp
  (params (Key :type Key%20Structure :default "None"))
  (bind _scenecapturecomponent2d (Variables|Default|GetSceneCaptureComponent2D))
  ;[0.1667 0.1667 0.1667] Move Item
  (:Pressed
    (Variables|/Script/Engine.SceneCaptureComponent2D|SetFOVAngle _scenecapturecomponent2d (Math|Float|Clamp(Float) (- (Variables|/Script/Engine.SceneCaptureComponent2D|GetFOVAngle _scenecapturecomponent2d) 3.0) 3e+01 8e+01))))

(fn ConstructionScript)