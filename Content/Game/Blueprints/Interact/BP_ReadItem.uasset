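; BP_ReadItem is an actor that shows a readable text popup when the player reads an item.
; Read creates a W_ReadItem widget with the given title and content, then moves input from the player to itself.
; Pressing IA_Interact returns input to the player, removes the widget and destroys the actor if the widget is valid.
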(event Input|EnhancedActionEvents|EnhancedInputActionIA_Interact
  (params (ActionValue :type Boolean) (ElapsedSeconds :type Float%20%28double-precision%29) (TriggeredSeconds :type Float%20%28double-precision%29) (InputAction :type Input%20Action%20Object%20Reference :default "/Game/Game/Input/Actions/IA_Interact.IA_Interact"))
  (bind _returnvalue (Game|GetPlayerController 0))
  ;[0.1042 0.1042 0.1042] Close Widget
  (Input|DisableInput _returnvalue)
  (Input|EnableInput (Variables|Default|GetPlayer) _returnvalue)
  (Utilities|IsValid (Variables|Default|GetRead%20Widget)
    (:Is%20Valid
      (Widget|RemovefromParent (Variables|Default|GetRead%20Widget))
      (Variables|Default|SetRead%20Widget 0)
      (Actor|DestroyActor))))

(event EventRead
  (params (Player :type Character%20Object%20Reference) (Title :type Text) (Content :type Text))
  (bind _returnvalue (Game|GetPlayerController 0))
  ;[0.1146 0.1146 0.1146] Create Widget
  (Variables|Default|SetPlayer Player)
  (bind _returnvalue_2 (UserInterface|CreateWidget "/Game/UI/Interact/Read/W_ReadItem.W_ReadItem_C" 0 Title Content))
  (bind _output_get (Variables|Default|SetRead%20Widget _returnvalue_2))
  (UserInterface|Viewport|AddtoViewport _output_get 0)
  (Input|DisableInput (Variables|Default|GetPlayer) _returnvalue)
  (Input|EnableInput _returnvalue))

(fn ConstructionScript)