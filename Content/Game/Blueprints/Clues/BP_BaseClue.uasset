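; Base clue actor that shows a prompt widget while the player is inside its collision sphere and opens a clue view when interacted with.
; Interact checks the Inspect, Read and InspectAndRead flags in that order and spawns the matching inspect, read or combined item actor far from the world origin.
; It passes that actor the player and the clue's text, plus mesh, rotation and scale for the inspect modes.
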(event OnComponentBeginOverlap(CollisionSphere)
  (params (OverlappedComponent :type Primitive%20Component%20Object%20Reference) (OtherActor :type Actor%20Object%20Reference) (OtherComp :type Primitive%20Component%20Object%20Reference) (OtherBodyIndex :type Integer) (bFromSweep :type Boolean) (SweepResult :type Hit%20Result%20Structure%20%28by%20ref%29))
  ;[0.03646 0.03646 0.03646] Display prompt
  (if (== OtherActor (Variables|Default|GetPlayer))
    (Rendering|SetVisibility (Variables|Default|GetWidget) true false)))

(event OnComponentEndOverlap(CollisionSphere)
  (params (OverlappedComponent :type Primitive%20Component%20Object%20Reference) (OtherActor :type Actor%20Object%20Reference) (OtherComp :type Primitive%20Component%20Object%20Reference) (OtherBodyIndex :type Integer))
  ;[0.03646 0.03646 0.03646] Display prompt
  (if (== OtherActor (Variables|Default|GetPlayer))
    (Rendering|SetVisibility (Variables|Default|GetWidget) false false)))

(event EventBeginPlay
  (bind _asbp_third_person_character (Utilities|Casting|CastToBP_ThirdPersonCharacter (Game|GetPlayerCharacter 0)))
  (Variables|Default|SetPlayer _asbp_third_person_character))

(event EventInteract
  (params (Player :type Character%20Object%20Reference))
  (if (Variables|Public|Interaction|Inspection|GetInspect?)
    ;[0.05208 0.05208 0.05208] Inspect
    (bind _returnvalue (Game|SpawnActorfromClass "/Game/Game/Blueprints/Interact/BP_InspectItem.BP_InspectItem_C" (Math|Transform|MakeTransform "100000000.000000,0.000000,0.000000") "Undefined" "MultiplyWithRoot" 0 0))
    (Default|SetRotationandScale _returnvalue (Variables|Public|Interaction|Inspection|GetRotation) (Variables|Public|Interaction|Inspection|GetScale))
    (Default|Inspect _returnvalue Player (Variables|/Script/Engine.StaticMeshComponent|GetStaticMesh (Variables|Default|GetStatic%20Mesh)) (Variables|Public|Interaction|Inspection|GetName) (Variables|Public|Interaction|Inspection|GetDescription))
    (elif (Variables|Public|Interaction|Read|GetRead?)
      ;[0.04688 0.04688 0.04688] Read
      (bind _returnvalue_2 (Game|SpawnActorfromClass "/Game/Game/Blueprints/Interact/BP_ReadItem.BP_ReadItem_C" (Math|Transform|MakeTransform "100000000.000000,0.000000,0.000000") "Undefined" "MultiplyWithRoot" 0 0))
      (Default|Read _returnvalue_2 Player (Variables|Public|Interaction|Read|GetTitle) (Variables|Public|Interaction|Read|GetContent))
      (elif (Variables|Public|Interaction|GetInspect%20and%20Read)
        ;[0.06771 0.06771 0.06771] Inspect and Read
        (bind _returnvalue_3 (Game|SpawnActorfromClass "/Game/Game/Blueprints/Interact/BP_InspectReadItem.BP_InspectReadItem_C" (Math|Transform|MakeTransform "100000000.000000,0.000000,0.000000") "Undefined" "MultiplyWithRoot" 0 0))
        (Default|SetRotationandScale _returnvalue_3 (Variables|Public|Interaction|Inspection|GetRotation) (Variables|Public|Interaction|Inspection|GetScale))
        (Default|InspectRead _returnvalue_3 Player (Variables|/Script/Engine.StaticMeshComponent|GetStaticMesh (Variables|Default|GetStatic%20Mesh)) (Variables|Public|Interaction|Inspection|GetName) (Variables|Public|Interaction|Inspection|GetDescription) (Variables|Public|Interaction|Read|GetTitle) (Variables|Public|Interaction|Read|GetContent))))))

(fn ConstructionScript)